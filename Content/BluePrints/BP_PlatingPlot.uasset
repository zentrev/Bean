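; Planting plot where the bean character can spend a bean to grow a beanstalk, once per plot.
; Overlapping the trigger while unplanted opens the UI_Beanstalk widget and shows the mouse cursor.
; Plant closes the widget, removes a bean of the given size from the player, and on success reveals a pre-placed stalk with collision and marks the plot planted.
; Size 0 shows the small stalk, while sizes 1 and 2 both show the medium one.
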(event `self.trigger.OnComponentBeginOverlap`
  (params (OverlappedComponent :type "PrimitiveComponent Object Reference") (OtherActor :type "Actor Object Reference") (OtherComp :type "PrimitiveComponent Object Reference") (OtherBodyIndex :type Integer) (bFromSweep :type Boolean) (SweepResult :type "HitResult Structure (by ref)"))
  (cast `/Game/Blueprints/BP_BeanCharacter` OtherActor)
  (if (not (`self.Planted`))
    (bind _returnvalue (`|CreateWidget` "/Game/UI/UI_Beanstalk.UI_Beanstalk_C"))
    (bind _output_get (set `self.widget` _returnvalue))
    (`UserWidget.AddToViewport` _output_get 0)
    (set `PlayerController.bShowMouseCursor` true (`GameplayStatics.GetPlayerController` 0))))

(fn `Plant`
  (params (player :type "BeanCharacter Object Reference") (size :type Integer))
  (bind _smallstalk (`self.SmallStalk`))
  (bind _medstalk (`self.MedStalk`))
  (bind _medstalk_2 (`self.MedStalk`))
  (`Widget.RemoveFromParent` (`self.widget`))
  (if (not (`self.Planted`))
    (bind _returnvalue (`BeanCharacter.RemoveBean` player size))
    (if _returnvalue
      (switch `int` size
        (:`0`
          (`SceneComponent.SetVisibility` _smallstalk true false)
          (`PrimitiveComponent.SetCollisionEnabled` _smallstalk "QueryAndPhysics"))
        (:`1`
          (`SceneComponent.SetVisibility` _medstalk true false)
          (`PrimitiveComponent.SetCollisionEnabled` _medstalk "QueryAndPhysics"))
        (:`2`
          (`SceneComponent.SetVisibility` _medstalk_2 true false)
          (`PrimitiveComponent.SetCollisionEnabled` _medstalk_2 "QueryAndPhysics")))
      (set `self.Planted` true))))

(fn `UserConstructionScript`)