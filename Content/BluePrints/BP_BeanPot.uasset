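; Interactive bean pot that grows beans over time, dries out without water, and can be watered or harvested by the player.
; Tick runs a watering timer that swaps the plant to its dry mesh, and a growth timer whose interval depends on dryness, with beans capped at a maximum.
; BeanCharacter overlap shows an options widget, whose validity gates the water and harvest inputs.
; Harvesting spawns BP_BeanPod actors and resets the count.
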(event `self.ReceiveBeginPlay`
  (set `self.GrowTimer` (`self.GrowTimerWatered`))
  (set `self.WaterTimer` (`self.WaterTimerReset`)))

(event `self.ReceiveActorBeginOverlap`
  (params (OtherActor :type "Actor Object Reference"))
  (bind _returnvalue (`GameplayStatics.GetPlayerController` 0))
  ;[1 1 1] UIDisplay
  (cast `BeanCharacter` OtherActor)
  (bind _returnvalue_2 (`|CreateWidget` "/Game/UI/UI_BeanPotOptions.UI_BeanPotOptions_C" _returnvalue self))
  (`UserWidget.AddToViewport` _returnvalue_2 0)
  (bind _output_get (set `self.BeanPotUIOptions` _returnvalue_2))
  (`WidgetBlueprintLibrary.SetInputMode_GameAndUIEx` _returnvalue _output_get "DoNotLock" false))

(event `self.ReceiveActorEndOverlap`
  (params (OtherActor :type "Actor Object Reference"))
  ;[1 1 1] UIDisplay
  (cast `BeanCharacter` OtherActor)
  (`/Engine/EditorBlueprintResources/StandardMacros.IsValid` (`self.BeanPotUIOptions`)
    (:`Is Valid`
      (`Widget.RemoveFromParent` (`self.BeanPotUIOptions`))
      (`WidgetBlueprintLibrary.SetInputMode_GameOnly` (`GameplayStatics.GetPlayerController` 0)))))

(event `InputAction|Action1`
  (params (Key :type "Key Structure"))
  ;[1 1 1] Inputs
  (:`Pressed`
    (`/Engine/EditorBlueprintResources/StandardMacros.IsValid` (`self.BeanPotUIOptions`)
      (:`Is Valid`
        (`self.HarvestBeans`)))))

(event `self.ReceiveTick`
  (params (DeltaSeconds :type "Float (single-precision)"))
  (`|ExecutionSequence`
    (:`then_0`
      ;[1 1 1] Watering
      (bind _output_get (set `self.WaterTimer` (- (`self.WaterTimer`) DeltaSeconds)))
      (if (<= _output_get 0.0)
        (set `self.NeedsWatering` true)
        (`StaticMeshComponent.SetStaticMesh` (`self.Plant`) (`self.DryMesh`))))
    (:`then_1`
      ;[1 1 1] BeanGrowth
      (bind _output_get_2 (set `self.GrowTimer` (- (`self.GrowTimer`) DeltaSeconds)))
      (if (<= _output_get_2 0.0)
        (`|ExecutionSequence`
          (:`then_0`
            (`/Engine/EditorBlueprintResources/StandardMacros.IncrementInt` (`self.BeansGrown`)
              (:`  `
                (if (> (`self.BeansGrown`) (`self.MaxBeans`))
                  (set `self.BeansGrown` (`self.MaxBeans`))))))
          (:`then_1`
            (if (`self.NeedsWatering`)
              (set `self.GrowTimer` (`self.GrowTimerDry`))
              (else
                (set `self.GrowTimer` (`self.GrowTimerWatered`))))))))))

(event `InputAction|Action2`
  (params (Key :type "Key Structure"))
  ;[1 1 1] Inputs
  (:`Pressed`
    (`/Engine/EditorBlueprintResources/StandardMacros.IsValid` (`self.BeanPotUIOptions`)
      (:`Is Valid`
        (`self.WaterPot`)))))

(fn `HarvestBeans`
  (if (> (`self.BeansGrown`) 0)
    (`KismetSystemLibrary.PrintString` "Harvested")
    (for _ (range (+ (`self.BeansGrown`) 1))
      (`|SpawnActorFromClass` "/Game/BluePrints/BP_BeanPod.BP_BeanPod_C" (`SceneComponent.K2_GetComponentToWorld` (`self.BeanSpawn`)) "Undefined" "OverrideRootScale" null null))
    (set `self.BeansGrown` 0)
    (else
      (`KismetSystemLibrary.PrintString` "No Beans..."))))

(fn `UserConstructionScript`)

(fn `WaterPot`
  (`KismetSystemLibrary.PrintString` "Watered")
  (if (`self.NeedsWatering`)
    (`StaticMeshComponent.SetStaticMesh` (`self.Plant`) (`self.HealthyMesh`))
    (set `self.NeedsWatering` false)
    (set `self.WaterTimer` (`self.WaterTimerReset`))))