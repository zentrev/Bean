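; BP_BeanPod is a bean pickup that adds a bean to a BeanCharacter on contact.
; On BeginPlay it picks a random BeanSize and scales the Pod from a separate random roll, so visual size need not match the stored value.
; When a BeanCharacter hits the Pod, it passes BeanSize to AddBean, plays a pickup sound, prints a message and destroys itself.
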(event `self.ReceiveBeginPlay`
  (bind _returnvalue (`KismetMathLibrary.RandomIntegerInRange` 0 2))
  (set `self.BeanSize` _returnvalue)
  (`SceneComponent.SetRelativeScale3D` (`self.Pod`) (`KismetMathLibrary.Conv_DoubleToVector` (* (+ (`KismetMathLibrary.Conv_IntToDouble` _returnvalue) 1.0) 0.15))))

(event `self.Pod.OnComponentHit`
  (params (HitComponent :type "PrimitiveComponent Object Reference") (OtherActor :type "Actor Object Reference") (OtherComp :type "PrimitiveComponent Object Reference") (NormalImpulse :type "Vector Structure") (Hit :type "HitResult Structure (by ref)"))
  (bind _asbean_character (cast `BeanCharacter` OtherActor))
  (`BeanCharacter.AddBean` _asbean_character (`self.BeanSize`))
  (`GameplayStatics.PlaySound2D` "/Game/Audio/Pickup.Pickup" 1.0 1.0 0.0 null null)
  (`KismetSystemLibrary.PrintString` "Added Bean")
  (`self.K2_DestroyActor`))

(fn `UserConstructionScript`)