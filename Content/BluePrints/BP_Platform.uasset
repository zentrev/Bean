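; BP_Platform is a one-way platform for BP_BeanCharacter that can also be dropped through.
; Each tick, it disables PlatformCollision while the player's capsule center is below the Point component's height, and otherwise enables it.
; Holding the Down input disables collision and suspends the height check; releasing it re-enables collision.
; The player reference comes from GetActorOfClass on BeginPlay.
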(event `self.ReceiveBeginPlay`
  ;[1 1 1] Start
  (bind _returnvalue (`GameplayStatics.GetActorOfClass` "/Game/BluePrints/BP_BeanCharacter.BP_BeanCharacter_C"))
  (set `self.Player` _returnvalue)
  (set `self.KeyDown` false))

(event `self.ReceiveTick`
  (params (DeltaSeconds :type "Float (single-precision)"))
  (bind _platformcollision (`self.PlatformCollision`))
  (bind (_returnvalue_x _returnvalue_y _returnvalue_z) (`KismetMathLibrary.BreakVector` (`SceneComponent.K2_GetComponentLocation` (`self.Point`))))
  (bind (_returnvalue_x_2 _returnvalue_y_2 _returnvalue_z_2) (`KismetMathLibrary.BreakVector` (`SceneComponent.K2_GetComponentLocation` (`Character.CapsuleComponent` (`self.Player`)))))
  ;[1 1 1] SetCollisions
  (if (`self.KeyDown`)
    _
    (elif (< _returnvalue_z_2 _returnvalue_z)
      (`PrimitiveComponent.SetCollisionEnabled` _platformcollision "NoCollision")
      (else
        (`PrimitiveComponent.SetCollisionEnabled` _platformcollision "QueryAndPhysics")))))

(event `InputAction|Down`
  (params (Key :type "Key Structure"))
  (bind _platformcollision (`self.PlatformCollision`))
  ;[1 1 1] Input Down
  (:`Pressed`
    (set `self.KeyDown` true)
    (`PrimitiveComponent.SetCollisionEnabled` _platformcollision "NoCollision"))
  (:`Released`
    (set `self.KeyDown` false)
    (`PrimitiveComponent.SetCollisionEnabled` _platformcollision "QueryAndPhysics")))

(fn `UserConstructionScript`)